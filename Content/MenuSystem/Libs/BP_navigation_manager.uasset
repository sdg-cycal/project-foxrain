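; Menu navigation manager that drives keyboard and gamepad focus through UI panels, keeping mouse hover in sync.
; Panels implementing KeyboardNavigablePanel register as steps in an array, each tracking its selected widget.
; OnInput asks the focused widget what each direction or enter key does, then moves selection, clicks, changes values or jumps by custom index.
; Escape tells panels above the focused step, or the focused one, to close, unless overridden.
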(fn `AddToNavigableArray`
  (params (`Nav Item` :type "/Game/MenuSystem/Structs/NavItemStruct Structure (by ref)"))
  (returns (`Final Array` :type "Array of /Game/MenuSystem/Structs/WidgetFix Structure"))
  (locals (tempWidgetArray :type "Array of /Game/MenuSystem/Structs/WidgetFix Structure") (tempPanelRef :type "Widget Object Reference") (tempEventHandler :type "/Game/MenuSystem/Libs/BP_navset_event_handler Object Reference") (tempIndex :type Integer))
  (bind (_panelreferance _navigablewidgets _selectedwidgetindex _navitemseventhandler) (break `/Game/MenuSystem/Structs/NavItemStruct` `Nav Item`))
  ;[1 1 1] Chek if the item can be navigated and add to array
  (set `local.tempIndex` 0)
  (`/Engine/EditorBlueprintResources/StandardMacros.IsValid` _panelreferance
    (:`Is Valid`
      (set `local.tempPanelRef` _panelreferance)
      (set `local.tempEventHandler` _navitemseventhandler)
      (if (`KismetSystemLibrary.DoesImplementInterface` _panelreferance "/Game/MenuSystem/Widgets/Interface/KeyboardNavigablePanel.KeyboardNavigablePanel_C")
        (for _array_element _navigablewidgets
          (bind _widget (break `/Game/MenuSystem/Structs/WidgetFix` _array_element))
          (if (`KismetSystemLibrary.DoesImplementInterface` _widget "/Game/MenuSystem/Widgets/Interface/KeyboardNavigable.KeyboardNavigable_C")
            (message `/Game/MenuSystem/Widgets/Interface/KeyboardNavigable.SetEventHandler` _widget (`local.tempEventHandler`))
            (message `/Game/MenuSystem/Widgets/Interface/KeyboardNavigable.SetIndex` _widget (`local.tempIndex`) (+ (`KismetArrayLibrary.Array_LastIndex` (`self.NavigableItemArray_raw`)) 1))
            (add `/Game/MenuSystem/Libs/BP_navset_event_handler.OnMouseHover` (`local.tempEventHandler`) (`|CreateDelegate` :!event `NavItemMouseHover`))
            (add `/Game/MenuSystem/Libs/BP_navset_event_handler.OnMouseUnhover` (`local.tempEventHandler`) (`|CreateDelegate` :!event `NavItemMouseUnhover`))
            (`KismetArrayLibrary.Array_AddUnique` (`local.tempWidgetArray`) _array_element)
            (`/Engine/EditorBlueprintResources/StandardMacros.IncrementInt` (`local.tempIndex`))))
        (bind _returnvalue (`KismetArrayLibrary.Array_Add` (`self.NavigableItemArray_raw`) (make `/Game/MenuSystem/Structs/NavItemStruct` (`local.tempPanelRef`) (`local.tempWidgetArray`) _selectedwidgetindex (`local.tempEventHandler`))))
        (message `/Game/MenuSystem/Widgets/Interface/KeyboardNavigablePanel.SetStepIndex` (`local.tempPanelRef`) _returnvalue)
        (`self.SetNavigationFocus` true _returnvalue)
        (return (`local.tempWidgetArray`))))))

(fn `CustomNavigation`
  (params (CustomAction :type String))
  (locals (tempActionParse :type "Array of String"))
  (bind _tempactionparse (`local.tempActionParse`))
  (bind _output_get (set `local.tempActionParse` (`KismetStringLibrary.ParseIntoArray` CustomAction)))
  (switch `int` (`KismetArrayLibrary.Array_Length` _output_get)
    (:`0`
      (`KismetSystemLibrary.PrintString` null "No Custom navigation command is provided" true true (struct :`R` 1.0 :`G` 0.431695 :`A` 1.0)) ; Reminder, in case forget to provide command
    )
    (:`1`
      (`self.NavigateTo` (`KismetStringLibrary.Conv_StringToInt` (`|GetArrayItem` (`local.tempActionParse`)))))
    (:`2`
      (switch `string` (`|GetArrayItem` _tempactionparse)
        (:`select`
          (`self.NavigateTo` (`KismetStringLibrary.Conv_StringToInt` (`|GetArrayItem` _tempactionparse 1))))))))

(fn `CycleFirst`
  (`self.SetNavigationFocus` false (`self.CurrentlyFocusedStep`))
  (setmembers `/Game/MenuSystem/Structs/NavItemStruct` :`StructRef` (`|GetArrayItem` (`self.NavigableItemArray_raw`) (`self.CurrentlyFocusedStep`)) :`Selected Widget Index` 0)
  (`self.SetNavigationFocus` true (`self.CurrentlyFocusedStep`)))

(fn `CycleLast`
  (bind _output (`|GetArrayItem` (`self.NavigableItemArray_raw`) (`self.CurrentlyFocusedStep`)))
  (`self.SetNavigationFocus` false (`self.CurrentlyFocusedStep`))
  (setmembers `/Game/MenuSystem/Structs/NavItemStruct` :`StructRef` _output :`Selected Widget Index` (`KismetArrayLibrary.Array_LastIndex` (`.NavigableWidgets_5_6E2081A042DEF7ED68953185A3D58380` (break `/Game/MenuSystem/Structs/NavItemStruct` _output))))
  (`self.SetNavigationFocus` true (`self.CurrentlyFocusedStep`)))

(fn `GetCurrentStep`
  (returns (CurrentStep :type Integer))
  (return (`self.CurrentlyFocusedStep`)))

(fn `GetNavigableItemList`
  (returns (NavigableItemArray :type "Array of /Game/MenuSystem/Structs/NavItemStruct Structure"))
  (return (`self.NavigableItemArray_raw`)))

(fn `GetNavItemsFromContainer`
  (params (Box :type "Widget Object Reference (by ref)") (`Is Horizontal/Vertical` :type Boolean))
  (returns (`Navigable Widgets` :type "Array of /Game/MenuSystem/Structs/WidgetFix Structure"))
  (locals (tempWidgetArray :type "Array of /Game/MenuSystem/Structs/WidgetFix Structure"))
  (if `Is Horizontal/Vertical`
    (bind `_as가로_박스` (cast `HorizontalBox` Box))
    (for _index (range (`PanelWidget.GetChildrenCount` `_as가로_박스`))
      (`KismetArrayLibrary.Array_Add` (`local.tempWidgetArray`) (make `/Game/MenuSystem/Structs/WidgetFix` (`PanelWidget.GetChildAt` `_as가로_박스` _index))))
    (else
      (bind `_as세로_박스` (cast `VerticalBox` Box))
      (for _index_2 (range (`PanelWidget.GetChildrenCount` `_as세로_박스`))
        (`KismetArrayLibrary.Array_Add` (`local.tempWidgetArray`) (make `/Game/MenuSystem/Structs/WidgetFix` (`PanelWidget.GetChildAt` `_as세로_박스` _index_2))))))
  (return (`local.tempWidgetArray`)))

(fn `Navigate`
  (params (PressedKey :type "Key Structure") (ExpectedKey :type "Array of Key Structure") (ActionType :type "/Game/MenuSystem/Enums/ENavActionTypes Enum" :default "NewEnumerator5") (CustomAction :type String))
  (if (`KismetArrayLibrary.Array_Contains` ExpectedKey PressedKey)
    (`|ExecutionSequence`
      (:`then_0`
        (switch `/Game/MenuSystem/Enums/ENavActionTypes` ActionType
          (:`NewEnumerator0`
            (`self.NavigateDown`))
          (:`NewEnumerator1`
            (`self.NavigateUp`))
          (:`NewEnumerator2`
            (`self.NavigateRight`))
          (:`NewEnumerator3`
            (`self.NavigateLeft`))
          (:`NewEnumerator4`
            (`self.SimulateClick`))
          (:`NewEnumerator6`
            (`self.CycleLast`))
          (:`NewEnumerator7`
            (`self.CycleFirst`))
          (:`NewEnumerator8`
            (`self.UpdateValue` true))
          (:`NewEnumerator9`
            (`self.UpdateValue` false))
          (:`NewEnumerator10`
            (`self.CustomNavigation` CustomAction))))
      (:`then_1`
        (`self.OnNavigation` (select `bool` (`KismetInputLibrary.Key_IsGamepadKey` PressedKey) :`false` (select `bool` (`KismetInputLibrary.Key_IsKeyboardKey` PressedKey) :`false` (select `bool` (`KismetInputLibrary.Key_IsMouseButton` PressedKey) :`false` "NewEnumerator3" :`true` "NewEnumerator2" :!type "/Game/MenuSystem/Enums/ENavigationDeviceTypes Enum") :`true` "NewEnumerator1") :`true` "NewEnumerator0"))))))

(fn `NavigateDown`
  (locals (tempPreviousFocusedWidget :type "/Game/MenuSystem/Structs/WidgetFix Structure"))
  (bind _output (`|GetArrayItem` (`self.NavigableItemArray_raw`) (`self.CurrentlyFocusedStep`)))
  (bind (_panelreferance _navigablewidgets _selectedwidgetindex) (break `/Game/MenuSystem/Structs/NavItemStruct` _output))
  (bind _returnvalue (+ _selectedwidgetindex 1))
  (if (>= (`KismetArrayLibrary.Array_LastIndex` _navigablewidgets) _returnvalue)
    (`self.SetNavigationFocus` false (`self.CurrentlyFocusedStep`))
    (setmembers `/Game/MenuSystem/Structs/NavItemStruct` :`StructRef` _output :`Selected Widget Index` _returnvalue)
    (`self.SetNavigationFocus` true (`self.CurrentlyFocusedStep`))))

(fn `NavigateLeft`)

(fn `NavigateRight`)

(fn `NavigateTo`
  (params (index :type Integer))
  (bind _currentlyfocusedstep (`self.CurrentlyFocusedStep`))
  (`self.SetNavigationFocus` false _currentlyfocusedstep)
  (setmembers `/Game/MenuSystem/Structs/NavItemStruct` :`StructRef` (`|GetArrayItem` (`self.NavigableItemArray_raw`) _currentlyfocusedstep) :`Selected Widget Index` index)
  (`self.SetNavigationFocus` true (`self.CurrentlyFocusedStep`)))

(fn `NavigateUp`
  (bind _output (`|GetArrayItem` (`self.NavigableItemArray_raw`) (`self.CurrentlyFocusedStep`)))
  (bind _returnvalue (- (`.SelectedWidgetIndex_12_CCC55F6E4DEDC51A992C498EF1CA1D4D` (break `/Game/MenuSystem/Structs/NavItemStruct` _output)) 1))
  (if (>= _returnvalue 0)
    (`self.SetNavigationFocus` false (`self.CurrentlyFocusedStep`))
    (setmembers `/Game/MenuSystem/Structs/NavItemStruct` :`StructRef` _output :`Selected Widget Index` _returnvalue)
    (`self.SetNavigationFocus` true (`self.CurrentlyFocusedStep`))))

(fn `NavItemMouseHover`
  (params (SelectedIndex :type Integer) (StepIndex :type Integer))
  (bind _navigableitemarray_raw (`self.NavigableItemArray_raw`))
  (if (`KismetArrayLibrary.Array_IsValidIndex` _navigableitemarray_raw StepIndex)
    (`self.SetNavigationFocus` false StepIndex)
    (setmembers `/Game/MenuSystem/Structs/NavItemStruct` :`StructRef` (`|GetArrayItem` _navigableitemarray_raw StepIndex) :`Selected Widget Index` SelectedIndex)
    (`self.SetNavigationFocus` true StepIndex)))

(fn `NavItemMouseUnhover`
  (params (selectedIndex :type Integer) (StepIndex :type Integer)))

(fn `OnInput`
  (params (Key :type "Key Structure"))
  (returns (ReturnValue :type "EventReply Structure"))
  (locals (tempPressedKey :type "Key Structure"))
  (bind _navigableitemarray_raw (`self.NavigableItemArray_raw`))
  (bind _currentlyfocusedstep (`self.CurrentlyFocusedStep`))
  (bind ((`NavigableWidgets_5_6E2081A042DEF7ED68953185A3D58380` _navigablewidgets) (`SelectedWidgetIndex_12_CCC55F6E4DEDC51A992C498EF1CA1D4D` _selectedwidgetindex)) (break `/Game/MenuSystem/Structs/NavItemStruct` (`|GetArrayItem` _navigableitemarray_raw _currentlyfocusedstep)))
  (bind _output_widget (break `/Game/MenuSystem/Structs/WidgetFix` (`|GetArrayItem` _navigablewidgets _selectedwidgetindex)))
  (bind _output_get (set `local.tempPressedKey` Key))
  (if (`KismetArrayLibrary.Array_Contains` (`|MakeArray` "Escape" "Gamepad_Special_Right" :!type "Key Structure") _output_get)
    (if (`self.OverrideEscape`)
      (`self.OnEscapeWhenOverrideEnabled`)
      (return (`WidgetBlueprintLibrary.Unhandled`))
      (else
        (`self.RemoveUnfocusedSteps` true)
        (`self.OnEscape`)
        (return (`WidgetBlueprintLibrary.Handled`))))
    (elif (`KismetArrayLibrary.Array_IsValidIndex` _navigableitemarray_raw _currentlyfocusedstep)
      (bind _action (message `/Game/MenuSystem/Widgets/Interface/KeyboardNavigable.GetNavigationAction` _output_widget))
      (bind (_onup _ondown _onright _onleft _onenter _customaction) (break `/Game/MenuSystem/Structs/NavItemActionStruct` _action))
      (bind (_onup_2 _ondown_2 _onright_2 _onleft_2 _onenter_2) (break `/Game/MenuSystem/Structs/NavItemCustomActionStruct` _customaction))
      (`self.Navigate` (`local.tempPressedKey`) (`|MakeArray` "Up" "W" "Gamepad_DPad_Up" "Gamepad_LeftStick_Up" :!type "Key Structure") _onup _onup_2)
      (`self.Navigate` (`local.tempPressedKey`) (`|MakeArray` "Down" "S" "Gamepad_DPad_Down" "Gamepad_LeftStick_Down" :!type "Key Structure") _ondown _ondown_2)
      (`self.Navigate` (`local.tempPressedKey`) (`|MakeArray` "Right" "D" "Gamepad_DPad_Right" "Gamepad_LeftStick_Right" :!type "Key Structure") _onright _onright_2)
      (`self.Navigate` (`local.tempPressedKey`) (`|MakeArray` "Left" "A" "Gamepad_DPad_Left" "Gamepad_LeftStick_Left" :!type "Key Structure") _onleft _onleft_2)
      (`self.Navigate` (`local.tempPressedKey`) (`|MakeArray` "Enter" "SpaceBar" "Gamepad_FaceButton_Bottom" "E" :!type "Key Structure") _onenter _onenter_2))))

(fn `Remove`
  (params (StepIndex :type Integer) (RemoveFromArrayOnly :type Boolean))
  (bind _currentlyfocusedstep (`self.CurrentlyFocusedStep`))
  (bind _navigableitemarray_raw (`self.NavigableItemArray_raw`))
  (if RemoveFromArrayOnly
    (`KismetArrayLibrary.Array_Remove` _navigableitemarray_raw StepIndex)
    (bind _output_get (set `self.CurrentlyFocusedStep` (`KismetMathLibrary.Clamp` (- StepIndex 1) 0 (`KismetArrayLibrary.Array_LastIndex` _navigableitemarray_raw))))
    (`self.SetNavigationFocus` true _output_get)
    (else
      (`self.SetNavigationFocus` false _currentlyfocusedstep)
      (`KismetArrayLibrary.Array_Remove` (`self.NavigableItemArray_raw`) StepIndex)
      (`self.SetNavigationFocus` true (`KismetMathLibrary.Clamp` (- _currentlyfocusedstep 1) 0 (`KismetArrayLibrary.Array_LastIndex` (`self.NavigableItemArray_raw`)))))))

(fn `RemoveUnfocusedSteps`
  (params (EscKeyPress :type Boolean))
  (bind _returnvalue (`KismetArrayLibrary.Array_LastIndex` (`self.NavigableItemArray_raw`)))
  (if (< _returnvalue 0)
    (return)
    (elif (> _returnvalue (`self.CurrentlyFocusedStep`))
      ;[1 1 1] last step should always be the focused step. but if that is not the case, remove any higher step than the current step
      (for _index (range (+ (`self.CurrentlyFocusedStep`) 1) (+ _returnvalue 1))
        (message `/Game/MenuSystem/Widgets/Interface/KeyboardNavigablePanel.OnEscapeInput` (`.PanelReferance_9_4E5BD57648F39432D5027DB78636F72C` (break `/Game/MenuSystem/Structs/NavItemStruct` (`|GetArrayItem` (`self.NavigableItemArray_raw`) _index)))))
      (return)
      (else
        ;[1 1 1] if player press escape key then call the on escape method on the current navigable panel
        (if EscKeyPress
          (message `/Game/MenuSystem/Widgets/Interface/KeyboardNavigablePanel.OnEscapeInput` (`.PanelReferance_9_4E5BD57648F39432D5027DB78636F72C` (break `/Game/MenuSystem/Structs/NavItemStruct` (`|GetArrayItem` (`self.NavigableItemArray_raw`) (`self.CurrentlyFocusedStep`)))))
          (return)
          (else
            (return)))))))

(fn `SetNavigationFocus`
  (params (`Focus Add/Clear` :type Boolean :default true) (StepIndex :type Integer))
  (bind _navigableitemarray_raw (`self.NavigableItemArray_raw`))
  (bind _currentlyfocusedstep (`self.CurrentlyFocusedStep`))
  (bind _navigableitemarray_raw_2 (`self.NavigableItemArray_raw`))
  (bind (_output_panelreferance _output_navigablewidgets _output_selectedwidgetindex) (break `/Game/MenuSystem/Structs/NavItemStruct` (`|GetArrayItem` _navigableitemarray_raw_2 _currentlyfocusedstep)))
  (bind ((`NavigableWidgets_5_6E2081A042DEF7ED68953185A3D58380` _navigablewidgets) (`SelectedWidgetIndex_12_CCC55F6E4DEDC51A992C498EF1CA1D4D` _selectedwidgetindex)) (break `/Game/MenuSystem/Structs/NavItemStruct` (`|GetArrayItem` _navigableitemarray_raw StepIndex)))
  (bind _output_widget (break `/Game/MenuSystem/Structs/WidgetFix` (`|GetArrayItem` _output_navigablewidgets _output_selectedwidgetindex)))
  (bind _widget (break `/Game/MenuSystem/Structs/WidgetFix` (`|GetArrayItem` _navigablewidgets _selectedwidgetindex)))
  (if (and (`KismetArrayLibrary.Array_IsValidIndex` _navigableitemarray_raw_2 _currentlyfocusedstep) (!= (`self.CurrentlyFocusedStep`) StepIndex))
    (message `/Game/MenuSystem/Widgets/Interface/KeyboardNavigable.RemoveFocus` _output_widget))
  (set `self.CurrentlyFocusedStep` StepIndex)
  (if (`KismetArrayLibrary.Array_IsValidIndex` _navigableitemarray_raw StepIndex)
    (if `Focus Add/Clear`
      (message `/Game/MenuSystem/Widgets/Interface/KeyboardNavigable.SetFocus` _widget)
      (else
        (message `/Game/MenuSystem/Widgets/Interface/KeyboardNavigable.RemoveFocus` _widget)))))

(fn `SetOverrideEscape`
  (params (OverrideEscape :type Boolean))
  (set `self.OverrideEscape` OverrideEscape)
  (`self.OnOverrideEscape`))

(fn `SimulateClick`
  (bind (_panelreferance _navigablewidgets _selectedwidgetindex) (break `/Game/MenuSystem/Structs/NavItemStruct` (`|GetArrayItem` (`self.NavigableItemArray_raw`) (`self.CurrentlyFocusedStep`))))
  (message `/Game/MenuSystem/Widgets/Interface/KeyboardNavigable.OnClick` (`.Widget_2_425509A44D85A122B67D7783D4133412` (break `/Game/MenuSystem/Structs/WidgetFix` (`|GetArrayItem` _navigablewidgets _selectedwidgetindex)))))

(fn `UpdateValue`
  (params (`Increase/Decrease` :type Boolean))
  (bind (_panelreferance _navigablewidgets _selectedwidgetindex) (break `/Game/MenuSystem/Structs/NavItemStruct` (`|GetArrayItem` (`self.NavigableItemArray_raw`) (`self.CurrentlyFocusedStep`))))
  (message `/Game/MenuSystem/Widgets/Interface/KeyboardNavigable.ChangeValue` (`.Widget_2_425509A44D85A122B67D7783D4133412` (break `/Game/MenuSystem/Structs/WidgetFix` (`|GetArrayItem` _navigablewidgets _selectedwidgetindex))) `Increase/Decrease`))
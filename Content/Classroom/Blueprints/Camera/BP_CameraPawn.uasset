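; Free-flying camera pawn that spawns a BP_SmoothCamera on BeginPlay and makes it the first player's view target.
; Movement and look axes ease speeds that move and rotate the pawn in local space each Tick, with roll self-levelling.
; The smooth camera trails the pawn's transform through TInterpTo, adding a second layer of smoothing.
; Strafing scales by RotationSpeed, while forward and vertical movement use MovementSpeed.
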(event `self.ReceiveBeginPlay`
  (bind _returnvalue (`|SpawnActorFromClass` "/Game/Classroom/Blueprints/Camera/BP_SmoothCamera.BP_SmoothCamera_C" (`self.GetTransform`) "Undefined" "OverrideRootScale" null null))
  (bind _output_get (set `self.SmoothCamera` _returnvalue))
  (`PlayerController.SetViewTargetWithBlend` (`GameplayStatics.GetPlayerController` 0) _output_get 0.0 "VTBlend_Linear" 0.0 false))

(event `self.ReceiveTick`
  (params (DeltaSeconds :type "Float (single-precision)"))
  (bind _returnvalue (`GameplayStatics.GetWorldDeltaSeconds`))
  (bind _returnvalue_2 (`GameplayStatics.GetWorldDeltaSeconds`))
  (`self.K2_SetActorTransform` (`self.SmoothCamera`) (`KismetMathLibrary.TInterpTo` (`self.GetTransform` (`self.SmoothCamera`)) (`self.GetTransform`) DeltaSeconds 1.0) false false)
  (`self.K2_AddActorLocalOffset` (`KismetMathLibrary.MakeVector` (* _returnvalue_2 (`self.CurrentForwardSpeed`)) (* _returnvalue_2 (`self.CurrentRightSpeed`)) (* _returnvalue_2 (`self.CurrentUpSpeed`))))
  (`self.K2_AddActorLocalRotation` (`KismetMathLibrary.MakeRotator` (* _returnvalue (`self.CurrentRollSpeed`)) (* (`self.CurrentPitchSpeed`) _returnvalue) (* (`self.CurrentYawSpeed`) _returnvalue))))

(event `InputAxis|MoveForward`
  (params (AxisValue :type "Float (single-precision)"))
  (set `self.CurrentForwardSpeed` (`KismetMathLibrary.FInterpTo` (`self.CurrentForwardSpeed`) (* AxisValue (`self.MovementSpeed`)) (`GameplayStatics.GetWorldDeltaSeconds`) 5.0)))

(event `InputAxis|MoveUp`
  (params (AxisValue :type "Float (single-precision)"))
  (set `self.CurrentUpSpeed` (`KismetMathLibrary.FInterpTo` (`self.CurrentUpSpeed`) (* AxisValue (`self.MovementSpeed`)) (`GameplayStatics.GetWorldDeltaSeconds`) 5.0)))

(event `InputAxis|MoveRight`
  (params (AxisValue :type "Float (single-precision)"))
  (set `self.CurrentRightSpeed` (`KismetMathLibrary.FInterpTo` (`self.CurrentRightSpeed`) (* AxisValue (`self.RotationSpeed`)) (`GameplayStatics.GetWorldDeltaSeconds`) 5.0)))

(event `InputAxis|LookUp`
  (params (AxisValue :type "Float (single-precision)"))
  (bind _returnvalue_roll (`KismetMathLibrary.BreakRotator` (`self.K2_GetActorRotation`)))
  (set `self.CurrentPitchSpeed` (`KismetMathLibrary.FInterpTo` (`self.CurrentPitchSpeed`) (* AxisValue (`self.RotationSpeed`)) (`GameplayStatics.GetWorldDeltaSeconds`) 5.0))
  (set `self.CurrentRollSpeed` (`KismetMathLibrary.FInterpTo` (`self.CurrentRollSpeed`) (* _returnvalue_roll -5.0) (`GameplayStatics.GetWorldDeltaSeconds`))))

(event `InputAxis|Turn`
  (params (AxisValue :type "Float (single-precision)"))
  (set `self.CurrentYawSpeed` (`KismetMathLibrary.FInterpTo` (`self.CurrentYawSpeed`) (* AxisValue (`self.RotationSpeed`)) (`GameplayStatics.GetWorldDeltaSeconds`) 5.0)))

(fn `UserConstructionScript`)
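; BP_SmoothCamera is a camera Blueprint that drives smooth autofocus depth of field from whatever the camera faces.
; Each Tick traces forward on the Camera channel and eases FocusLocation toward the hit distance.
; On a hit, that value becomes the focal distance of Circle DOF post-process settings on the camera.
; On a miss, FocusLocation is interpolated from InfinitFocusLocation toward itself, and post-process settings stay untouched.
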(event `self.ReceiveTick`
  (params (DeltaSeconds :type "Float (single-precision)"))
  (bind _camera (`self.Camera`))
  (bind _returnvalue (`SceneComponent.K2_GetComponentLocation` _camera))
  (bind (_outhit _returnvalue_2) (`KismetSystemLibrary.LineTraceSingle` _returnvalue (+ _returnvalue (* (`SceneComponent.GetForwardVector` _camera) 5000.0)) "TraceTypeQuery2"))
  (if _returnvalue_2
    (bind (_bblockinghit _binitialoverlap _time _distance _location _impactpoint _normal _impactnormal _physmat _hitactor _hitcomponent _hitbonename _bonename _hititem _elementindex _faceindex _tracestart) (`GameplayStatics.BreakHitResult` _outhit))
    (bind _output_get (set `self.Focus Location` (`KismetMathLibrary.FInterpTo` (`self.Focus Location`) (`KismetMathLibrary.VSize` (- _location _tracestart)) (`GameplayStatics.GetWorldDeltaSeconds`) 15.0)))
    (set `CameraComponent.PostProcessSettings` (make `PostProcessSettings` :`DepthOfFieldFstop` 1.0 :`DepthOfFieldFocalDistance` _output_get :`DepthOfFieldFocalRegion` 500.0 :`DepthOfFieldMethod` "DOFM_CircleDOF") (`self.Camera`))
    (else
      (set `self.Focus Location` (`KismetMathLibrary.FInterpTo` (`self.Infinit Focus Location`) (`self.Focus Location`) (`GameplayStatics.GetWorldDeltaSeconds`) 15.0)))))

(fn `UserConstructionScript`)
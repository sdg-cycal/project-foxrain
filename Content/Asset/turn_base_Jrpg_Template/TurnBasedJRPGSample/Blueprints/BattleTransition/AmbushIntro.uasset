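; AmbushIntro is a battle transition that plays a scripted wolf ambush cinematic before the fight.
; It places the first two enemy units at AmbushController spawn points, then uses timelines to move them in, snapping each to its saved battle transform.
; Delay-staggered sequence branches blend between per-wolf cameras and a final ambush camera.
; ShowAll reveals the third wolf and player units, closes the cinematic UI and signals transition end.
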(event `self.StartTransition`
  (bind _wolf1 (`self.wolf1`))
  (bind _wolf1spawnpoint (`/Game/Asset/turn_base_Jrpg_Template/TurnBasedJRPGSample/Blueprints/AmbushController.wolf1SpawnPoint` (`self.ambushController`)))
  ;[1 1 1] Start ambush transition
  (`GameplayStatics.PlaySound2D` "/Game/Asset/turn_base_Jrpg_Template/TurnBasedJRPGSample/Sounds/WolfHowl_CUE.WolfHowl_CUE" 1.0 1.0 0.0 null null)
  (bind _returnvalue (`|CreateWidget` "/Game/Asset/turn_base_Jrpg_Template/TurnBasedJRPGSample/Blueprints/UI/CinematicUI.CinematicUI_C"))
  (bind _output_get (set `self.cinematicUI` _returnvalue))
  (`UserWidget.AddToViewport` _output_get 0)
  (`/Game/Asset/turn_base_Jrpg_Template/TurnBasedJRPGSample/Blueprints/UI/CinematicUI.PlayCinematicUI` (`self.cinematicUI`) true)
  (`KismetSystemLibrary.Delay` 0.2)
  (bind _outactors (`GameplayStatics.GetAllActorsOfClass` "/Game/Asset/turn_base_Jrpg_Template/TurnBasedJRPGSample/Blueprints/AmbushController.AmbushController_C"))
  (set `self.ambushController` (`|GetArrayItem` _outactors))
  (set `self.wolf1` (cast `` (`|GetArrayItem` (`/Game/Asset/turn_base_Jrpg_Template/TurnBasedJRPGSample/Blueprints/BattleTransition/AmbushIntro.enemyUnits` (`self.battle`))) :!pure true))
  (set `self.wolf2` (cast `` (`|GetArrayItem` (`/Game/Asset/turn_base_Jrpg_Template/TurnBasedJRPGSample/Blueprints/BattleTransition/AmbushIntro.enemyUnits` (`self.battle`)) 1) :!pure true))
  (set `self.wolf3` (cast `` (`|GetArrayItem` (`/Game/Asset/turn_base_Jrpg_Template/TurnBasedJRPGSample/Blueprints/BattleTransition/AmbushIntro.enemyUnits` (`self.battle`)) 2) :!pure true))
  (set `self.wolf1FinalTransform` (`self.GetTransform` (`self.wolf1`)))
  (`self.K2_SetActorLocationAndRotation` (`self.wolf1`) (`self.K2_GetActorLocation` _wolf1spawnpoint) (`self.K2_GetActorRotation` _wolf1spawnpoint) false false)
  (`self.DisableActor` _wolf1)
  (`PlayerController.SetViewTargetWithBlend` (`GameplayStatics.GetPlayerController` 0) (`ChildActorComponent.ChildActor` (`/Game/Asset/turn_base_Jrpg_Template/TurnBasedJRPGSample/Blueprints/BattleTransition/AmbushIntro.AmbushCamera` _wolf1)) 1.0 "VTBlend_Cubic" 0.0 false)
  (`KismetSystemLibrary.Delay` 1.0)
  (`|ExecutionSequence`
    (:`then_0`
      (`KismetSystemLibrary.Delay` 0.3)
      (`GameplayStatics.PlaySound2D` "/Game/Asset/turn_base_Jrpg_Template/TurnBasedJRPGSample/Sounds/WolfBite_CUE.WolfBite_CUE" 1.0 1.0 0.0 null null)
      (`GameplayStatics.PlaySound2D` "/Game/Asset/turn_base_Jrpg_Template/TurnBasedJRPGSample/Sounds/WolfSnarl_CUE.WolfSnarl_CUE" 1.0 1.0 0.0 null null))
    (:`then_1`
      (bind _animationduration (`self.PlayAnimation` (`self.wolf1`) "/Game/Asset/turn_base_Jrpg_Template/QuadrapedCreatures/Barghest/Animations/BARGHEST_run.BARGHEST_run" false))
      (`KismetSystemLibrary.Delay` _animationduration)
      (`self.PlayAnimation` (`self.wolf1`) "/Game/Asset/turn_base_Jrpg_Template/QuadrapedCreatures/Barghest/Animations/BARGHEST_walk.BARGHEST_walk" true))
    (:`then_2`
      (`self.ShowWolf1Intro`))
    (:`then_3`
      (`KismetSystemLibrary.Delay` 2.0)
      (`self.ShowWolf2Intro`))
    (:`then_4`
      (`KismetSystemLibrary.Delay` 4.0)
      (`self.ShowAll`))))

(event `ShowWolf1Intro`
  (bind (_wolf1finaltransform_location _wolf1finaltransform_rotation) (`KismetMathLibrary.BreakTransform` (`self.wolf1FinalTransform`)))
  (bind _wolf1spawnpoint (`/Game/Asset/turn_base_Jrpg_Template/TurnBasedJRPGSample/Blueprints/AmbushController.wolf1SpawnPoint` (`self.ambushController`)))
  (bind _returnvalue (`self.K2_GetActorLocation` _wolf1spawnpoint))
  ;[1 1 1] Move wolf 1
  (bind (_direction _alpha) (`Timeline|Wolf1MoveOverTime` :`NewTime` 0.0 :!via `PlayFromStart`)
    (:`Update`
      (`self.K2_SetActorLocation` (`self.wolf1`) (`KismetMathLibrary.VLerp` _returnvalue (+ _returnvalue (* (`self.GetActorForwardVector` _wolf1spawnpoint) 750.0)) _alpha) false false))
    (:`Finished`
      (`self.K2_SetActorLocationAndRotation` (`self.wolf1`) _wolf1finaltransform_location _wolf1finaltransform_rotation false false)
      (`self.PlayAnimation` (`self.wolf1`) "/Game/Asset/turn_base_Jrpg_Template/QuadrapedCreatures/Barghest/Animations/BarghestIntroIdle.BarghestIntroIdle" false))))

(event `ShowWolf2Intro`
  (bind _wolf2finaltransform_location (`KismetMathLibrary.BreakTransform` (`self.wolf2FinalTransform`)))
  (bind (_wolf2finaltransform_location_2 _wolf2finaltransform_rotation) (`KismetMathLibrary.BreakTransform` (`self.wolf2FinalTransform`)))
  (bind _wolf2 (`self.wolf2`))
  (bind _wolf2spawnpoint (`/Game/Asset/turn_base_Jrpg_Template/TurnBasedJRPGSample/Blueprints/AmbushController.wolf2SpawnPoint` (`self.ambushController`)))
  ;[1 1 1] Move wolf 2
  (set `self.wolf2FinalTransform` (`self.GetTransform` (`self.wolf2`)))
  (`self.K2_SetActorLocationAndRotation` (`self.wolf2`) (`self.K2_GetActorLocation` _wolf2spawnpoint) (`self.K2_GetActorRotation` _wolf2spawnpoint) false false)
  (`self.DisableActor` _wolf2)
  (`PlayerController.SetViewTargetWithBlend` (`GameplayStatics.GetPlayerController` 0) (`ChildActorComponent.ChildActor` (`/Game/Asset/turn_base_Jrpg_Template/TurnBasedJRPGSample/Blueprints/BattleTransition/AmbushIntro.AmbushCamera` _wolf2)) 1.0 "VTBlend_Cubic" 0.0 false)
  (`KismetSystemLibrary.Delay` 0.5)
  (`self.PlayAnimation` (`self.wolf2`) "/Game/Asset/turn_base_Jrpg_Template/QuadrapedCreatures/Barghest/Animations/BARGHEST_walk.BARGHEST_walk" true)
  (bind (_direction _alpha) (`Timeline|Wolf2MoveOverTime` :!via `PlayFromStart`)
    (:`Update`
      (`self.K2_SetActorRelativeLocation` (`self.wolf2`) (`KismetMathLibrary.VLerp` (`self.K2_GetActorLocation` (`/Game/Asset/turn_base_Jrpg_Template/TurnBasedJRPGSample/Blueprints/AmbushController.wolf2SpawnPoint` (`self.ambushController`))) _wolf2finaltransform_location _alpha) false false))
    (:`Finished`
      (`self.K2_SetActorLocationAndRotation` (`self.wolf2`) _wolf2finaltransform_location_2 _wolf2finaltransform_rotation false false)
      (`self.PlayAnimation` (`self.wolf2`) "/Game/Asset/turn_base_Jrpg_Template/QuadrapedCreatures/Barghest/Animations/BarghestIntroIdle.BarghestIntroIdle" false))))

(event `ShowAll`
  ;[1 1 1] Show all units
  (`PlayerController.SetViewTargetWithBlend` (`GameplayStatics.GetPlayerController` 0) (`/Game/Asset/turn_base_Jrpg_Template/TurnBasedJRPGSample/Blueprints/AmbushController.ambushCamera` (`self.ambushController`)) 1.0 "VTBlend_Cubic" 0.0 false)
  (`self.DisableActor` (`self.wolf3`))
  (`self.PlayAnimation` (`self.wolf3`) "/Game/Asset/turn_base_Jrpg_Template/QuadrapedCreatures/Barghest/Animations/BarghestIntroIdle.BarghestIntroIdle" false)
  (for _array_element (`/Game/Asset/turn_base_Jrpg_Template/TurnBasedJRPGSample/Blueprints/BattleTransition/AmbushIntro.playerUnits` (`self.battle`))
    (`self.DisableActor` _array_element)
    (`self.PlayAnimation` _array_element (`/Game/Asset/turn_base_Jrpg_Template/TurnBasedJRPGSample/Blueprints/BattleTransition/AmbushIntro.idleAnimation` _array_element) true))
  (`KismetSystemLibrary.Delay` 2.0)
  (`/Game/Asset/turn_base_Jrpg_Template/TurnBasedJRPGSample/Blueprints/UI/CinematicUI.PlayCinematicUI` (`self.cinematicUI`) false)
  (`self.OnTransitionEnded`))

(fn `UserConstructionScript`
  (`parent.UserConstructionScript`))
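; Battle transition actor that plays a glass-shatter effect with sound, then signals that the transition has ended.
; StartTransition snaps a SceneCaptureComponent2D to the player camera, captures the current view once and shows the GlassShatterUI widget.
; After a short delay it removes the widget, starts a camera fade from full opacity and immediately calls OnTransitionEnded without waiting for the fade.
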(event `self.StartTransition`
  ;[1 1 1] Shatter glass transition
  (`GameplayStatics.PlaySound2D` "/Game/Asset/turn_base_Jrpg_Template/TurnBasedJRPGSample/Sounds/GlassShatter_CUE.GlassShatter_CUE" 1.0 1.0 0.0 null null)
  (`SceneComponent.K2_SetWorldTransform` (`self.SceneCaptureComponent2D`) (`self.GetTransform` (`PlayerController.PlayerCameraManager` (`GameplayStatics.GetPlayerController` 0))) false false)
  (`SceneCaptureComponent2D.CaptureScene` (`self.SceneCaptureComponent2D`))
  (bind _returnvalue (`|CreateWidget` "/Game/Asset/turn_base_Jrpg_Template/TurnBasedJRPGSample/Blueprints/UI/GlassShatterUI.GlassShatterUI_C"))
  (`UserWidget.AddToViewport` _returnvalue 0)
  (`KismetSystemLibrary.Delay` 1.0)
  (`Widget.RemoveFromParent` _returnvalue)
  (`PlayerCameraManager.StartCameraFade` :`self` (`PlayerController.PlayerCameraManager` (`GameplayStatics.GetPlayerController` 0)) :`FromAlpha` 1.0 :`Duration` 0.5 :`bHoldWhenFinished` true)
  (`self.OnTransitionEnded`))

(fn `UserConstructionScript`
  (`parent.UserConstructionScript`))
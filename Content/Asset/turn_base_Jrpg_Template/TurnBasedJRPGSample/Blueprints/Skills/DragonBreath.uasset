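; DragonBreath is a turn-based battle skill in which the dragon spreads fire and damages every player unit.
; UseSkill runs timed parallel chains: the attacker's fire animation returning to idle, a camera blend to the DragonBattleController's breath camera with audio, and delayed damage.
; Damage loops backwards over PlayerUnits, setting each as current target for DealDamage, then fades audio and signals skill completion.
; The previous view target is saved but not restored here.
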(event `self.UseSkill`
  (bind _battlecontroller (`self.battleController`))
  (bind _currentattackingunit (`/Game/Asset/turn_base_Jrpg_Template/TurnBasedJRPGSample/Blueprints/Skills/DragonBreath.currentAttackingUnit` (`self.battleController`)))
  ;[1 1 1] Dragon spreads fire and damages all player units
  (bind _animationduration (`self.PlayAnimation` (`/Game/Asset/turn_base_Jrpg_Template/TurnBasedJRPGSample/Blueprints/Skills/DragonBreath.currentAttackingUnit` (`self.battleController`)) "/Game/Asset/turn_base_Jrpg_Template/QuadrapedCreatures/MountainDragon/Animations/ANIM_MOUNTAIN_DRAGON_FlyStationarySpreadFire.ANIM_MOUNTAIN_DRAGON_FlyStationarySpreadFire" false))
  (`|ExecutionSequence`
    (:`then_0`
      (`KismetSystemLibrary.Delay` _animationduration)
      (`self.PlayAnimation` _currentattackingunit (`/Game/Asset/turn_base_Jrpg_Template/TurnBasedJRPGSample/Blueprints/Skills/DragonBreath.idleAnimation` _currentattackingunit) true))
    (:`then_1`
      (bind _outactors (`GameplayStatics.GetAllActorsOfClass` "/Game/Asset/turn_base_Jrpg_Template/TurnBasedJRPGSample/Blueprints/DragonBattleController.DragonBattleController_C"))
      (`KismetSystemLibrary.Delay` 0.2)
      (bind _output_get (set `self.dragonBreathCamera` (`/Game/Asset/turn_base_Jrpg_Template/TurnBasedJRPGSample/Blueprints/DragonBattleController.dragonBreathCamera` (`|GetArrayItem` _outactors))))
      (set `self.defaultViewTarget` (`Controller.GetViewTarget` (`GameplayStatics.GetPlayerController` 0)))
      (`PlayerController.SetViewTargetWithBlend` (`GameplayStatics.GetPlayerController` 0) _output_get 3.0 "VTBlend_Cubic" 0.0 false)
      (`KismetSystemLibrary.Delay` 0.5)
      (`AudioComponent.Play` (`self.Audio`) 0.0))
    (:`then_2`
      (`KismetSystemLibrary.Delay` 3.5)
      (bind (_arrayindex _arrayelement) (`/Engine/EditorBlueprintResources/StandardMacros.ReverseForEachLoop` (`/Game/Asset/turn_base_Jrpg_Template/TurnBasedJRPGSample/Blueprints/Skills/DragonBreath.playerUnits` (`/Game/Asset/turn_base_Jrpg_Template/TurnBasedJRPGSample/Blueprints/Skills/DragonBreath.currentBattle` (`self.battleController`))))
        (:`LoopBody`
          (set `/Game/Asset/turn_base_Jrpg_Template/TurnBasedJRPGSample/Blueprints/Skills/DragonBreath.currentTargetUnit` _arrayelement _battlecontroller)
          (`self.DealDamage` _battlecontroller 0 (`self.damageMultiplier`)))
        (:`Completed`
          (`AudioComponent.FadeOut` (`self.Audio`) 1.0 0.0)
          (`KismetSystemLibrary.Delay` 1.0)
          (`self.OnSkillUsed`))))))

(fn `UserConstructionScript`
  (`parent.UserConstructionScript`))
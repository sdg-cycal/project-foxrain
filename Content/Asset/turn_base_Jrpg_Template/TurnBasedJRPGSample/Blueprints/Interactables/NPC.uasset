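; Interactable NPC for the turn-based JRPG sample that shows a sample conversation dialogue when the player interacts with it.
; It binds to an interaction detector from its child actor, enabling interaction on load and again after each use.
; Interacting blocks player input and opens the Conversation2D sample widget.
; When the conversation ends, input is restored, and a Yes answer opens the Conversation2D plugin's marketplace page.
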(event `self.ReceiveBeginPlay`
  ;[1 1 1] Display sample conversation dialogue
  (bind _asbp_interaction_detector (cast `` (`ChildActorComponent.ChildActor` (`self.Interaction`))))
  (set `self.interactionDetector` null _asbp_interaction_detector)
  (add `self.OnInteracted` (`.interactionDetector` (`self.interactionDetector`)) (delegate `OnInteractedHandler`))
  (add `self.OnLoaded` (`.interactionDetector` (`self.interactionDetector`)) (delegate `OnLoadedHandler`)))

(event `OnLoadedHandler`
  ;[1 1 1] Display sample conversation dialogue
  (`self.EnableInteraction` (`.interactionDetector` (`self.interactionDetector`))))

(event `OnInteractedHandler`
  ;[1 1 1] Display sample conversation dialogue
  (`self.EnableInteraction` (`.interactionDetector` (`self.interactionDetector`)))
  (`self.BlockPlayerInput` (`.AsBP JRPGCharacter Base` (cast `` (`GameplayStatics.GetPlayerPawn` 0) :!pure true)) true)
  (bind _returnvalue (`|CreateWidget` "/Game/Asset/turn_base_Jrpg_Template/TurnBasedJRPGSample/Blueprints/UI/Conversation2DSampleUI.Conversation2DSampleUI_C"))
  (`UserWidget.AddToViewport` _returnvalue 0)
  (add `/Game/Asset/turn_base_Jrpg_Template/TurnBasedJRPGSample/Blueprints/UI/Conversation2DSampleUI.OnConversationEnded` _returnvalue (delegate `OnConversationEndedHandler`)))

(event `OnConversationEndedHandler`
  (params (isYes :type Boolean))
  ;[1 1 1] Display sample conversation dialogue
  (`self.BlockPlayerInput` (`.AsBP JRPGCharacter Base` (cast `` (`GameplayStatics.GetPlayerPawn` 0) :!pure true)) false)
  (if isYes
    (bind _returnvalue (`KismetSystemLibrary.CanLaunchURL` "https://www.unrealengine.com/marketplace/en-US/slug/conversation2d-plugin"))
    (if _returnvalue
      (`KismetSystemLibrary.LaunchURL` "https://www.unrealengine.com/marketplace/en-US/slug/conversation2d-plugin"))))

(fn `UserConstructionScript`)
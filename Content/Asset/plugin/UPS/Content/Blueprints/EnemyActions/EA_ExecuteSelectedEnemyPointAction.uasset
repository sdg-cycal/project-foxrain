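; Enemy action that has the character execute the action on its selected enemy point.
; On start it calls StartEnemyPointAction on the Point, passing the character, and finishes when the point's completion callback fires.
; An abort is forwarded to the point, and either start or abort finishes immediately if the point is invalid.
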(event `self.InternalStartAction`
  (params (InCharacter :type "Character Object Reference"))
  (`self.Point`
    (:`then`
      (`UPSEnemyPointAction.StartEnemyPointAction` (`self.Point`) (delegate `CustomEvent_0`) (`self.Character`)))
    (:`else`
      (`self.FinishAction`))))

(event `CustomEvent_0`
  (params (EnemyPointAction :type "UPSEnemyPointAction Object Reference") (Character :type "Character Object Reference"))
  (`self.FinishAction`))

(event `self.InternalAbortAction`
  (params (InCharacter :type "Character Object Reference"))
  (bind _point (`self.Point`)
    (:`then`
      (`UPSEnemyPointAction.AbortEnemyPointAction` _point InCharacter))
    (:`else`
      (`self.FinishAction`))))
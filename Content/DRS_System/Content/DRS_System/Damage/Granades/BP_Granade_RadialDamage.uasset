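; BP_Granade_RadialDamage is a grenade Blueprint in the DRS damage system that deals area damage when it explodes.
; On the explosion event it applies full radial damage without falloff at its location, using the grenade's damage value, explosion radius and damage type.
; The owner of the causer manager component is excluded from the blast, and the instigator's controller is credited for the damage.
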(event `self.OnExplosion`
  (`GameplayStatics.ApplyRadialDamage` (`self.Get Granade Damage Value`) (`self.K2_GetActorLocation`) (`self.ExplosionsRadius`) (`self.DamageType`) (`|MakeArray` (`ActorComponent.GetOwner` (`self.CauserManagerComponent`))) self (`Pawn.GetController` (`self.GetInstigator`)) true))

(fn `UserConstructionScript`
  (`parent.UserConstructionScript`))
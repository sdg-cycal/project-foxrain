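; Base grenade actor for the DRS damage system that explodes on the server after a fuse delay and destroys itself on non-server instances at BeginPlay.
; Detonation calls an empty OnExplosion hook, multicasts an optionally radius-scaled emitter, destroys the actor and can draw a debug sphere.
; A helper computes damage from the damage class average, curve-scaled by the instigator's GameplayEffects level.
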(event `self.ReceiveBeginPlay`
  (if (`KismetSystemLibrary.IsServer`)
    (`KismetSystemLibrary.Delay` (`self.ExplosionDelay`))
    (`|ExecutionSequence`
      (:`then_0`
        ;[1 0 0.1807] OnExplosion
        (`self.OnExplosion`)
        (`/Engine/EditorBlueprintResources/StandardMacros.IsValid` (`self.ExplosionEffectEmitter`)
          (:`Is Valid`
            ;[1 0 0.1807] Spawn Emitter
            (`self.MULTICAST // Spawn Emiter`))
          (:`Is Not Valid`
            _))
        ;[1 0 0.1807] DestroyActor
        (`self.K2_DestroyActor`))
      (:`then_1`
        ;[1 0 0.1807] Draw Debug
        (if (`self.DrawDebug`)
          (`self.DrawDebugEvent`))))
    (else
      (`self.K2_DestroyActor`))))

(event `DrawDebugEvent`
  ;[0.3308 0 1] Draw Debug Event
  (`KismetSystemLibrary.DrawDebugSphere` (`self.K2_GetActorLocation`) (`self.ExplosionsRadius`) 20 (struct :`R` 0.330762 :`B` 1.0 :`A` 1.0) 1.0 1.0))

(event `OnExplosion`
  ;[0.3308 0 1] OnExplosion
)

(event `MULTICAST // Spawn Emiter`
  (bind _returnvalue (/ (`self.ExplosionsRadius`) 100.0))
  ;[0.1583 0.2487 1] MULTICAST // Spawn Emitter
  (`GameplayStatics.SpawnEmitterAtLocation` (`self.ExplosionEffectEmitter`) (`self.K2_GetActorLocation`) (struct) (select `bool` (`self.ScaleEmitterWithRadius`) :`false` (1.0 1.0 1.0) :`true` (`KismetMathLibrary.MakeVector` _returnvalue _returnvalue _returnvalue) :!type "Vector Structure")))

(fn `Get Granade Damage Value`
  (returns (ReturnValue :type "Float (double-precision)"))
  (return (`/Game/DRS_System/Content/DRS_System/DRS_FunctionLibrary.Apply Scaling To Float Value` (`/Game/DRS_System/Content/DRS_System/DRS_FunctionLibrary.Get Damage Value Average from class` (`self.CauserManagerComponent`) (`self.DamageType`)) "/Game/DRS_System/Content/DRS_System/Damage/Granades/Curve_GranadeDamageScaling.Curve_GranadeDamageScaling" (`/Game/DRS_System/Content/DRS_System/Gameplay/C_GameplayEffects.Get Level` (`self.GetComponentByClass` (`self.Instigator`) "/Game/DRS_System/Content/DRS_System/Gameplay/C_GameplayEffects.C_GameplayEffects_C")))))

(fn `UserConstructionScript`)
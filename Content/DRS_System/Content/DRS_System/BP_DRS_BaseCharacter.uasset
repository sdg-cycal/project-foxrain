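; Base character Blueprint for the DRS system that keeps max walk speed in step with gameplay effect modifiers.
; The server caches the starting speed, binds to an optional inventory component's base-value changes, and prefers that component's base speed.
; Modifier changes trigger a server-side recalculation from base speed and active modifiers, floored at zero.
; A multicast manually replicates the result to clients to prevent movement "teleporting".
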(event `self.ReceiveBeginPlay`
  (bind _returnvalue (`self.GetComponentByClass` "/Game/DRS_System/Content/InventorySystem/C_Inventory_Base.C_Inventory_Base_C"))
  ;[0 1 0.3583] Event Begin Play
  ;[1 0 0.1807] Save the inital WalkSpeed as BaseWalkSpeed
  (`self.Is Server?`
    (:`true`
      (set `self.BaseMaxWalkSpeed` (`CharacterMovementComponent.MaxWalkSpeed` (`self.CharacterMovement`)))
      ;[1 0 0.1807] Inventory Integration
      (`/Engine/EditorBlueprintResources/StandardMacros.IsValid` _returnvalue
        (:`Is Valid`
          (bind _output_get (set `self.Inventory Reference` _returnvalue))
          (add `/Game/DRS_System/Content/InventorySystem/C_Inventory_Base.OnBaseValueChange` _output_get (`|CreateDelegate` :!event `Recalculate Value`)))))))

(event `self.C_GameplayEffects.OnModifierChange`
  (params (Value :type "/Game/DRS_System/Content/_Global/E_ModifiableValues Enum" :default "NewEnumerator0") (`Value Spezification` :type Byte))
  ;[0.3308 0 1] OnModifierChange
  (`self.Recalculate Value` Value `Value Spezification`))

(event `MULTICAST // Recalculate WalkSpeed`
  (params (MaxWalkSpeed :type "Float (double-precision)"))
  ;[0.0812 0 1] Change WalkSpeed on Client (Manual Replication)
  (set `CharacterMovementComponent.MaxWalkSpeed` MaxWalkSpeed (`self.CharacterMovement`)))

(fn `Get BaseMaxWalkSpeed`
  (returns (ReturnValue :type "Float (double-precision)"))
  (bind _inventory_reference (`self.Inventory Reference`))
  (`/Engine/EditorBlueprintResources/StandardMacros.IsValid` _inventory_reference
    (:`Is Valid`
      (return (`/Game/DRS_System/Content/InventorySystem/C_Inventory_Base.Get BaseMaxWalkSpeed` _inventory_reference)))
    (:`Is Not Valid`
      (return (`self.BaseMaxWalkSpeed`)))))

(fn `Recalculate Value`
  (params (Value :type "/Game/DRS_System/Content/_Global/E_ModifiableValues Enum" :default "NewEnumerator0") (Spezification :type Byte))
  (`self.Is Server?`
    (:`true`
      (switch `/Game/DRS_System/Content/_Global/E_ModifiableValues` Value
        (:`NewEnumerator9`
          (`self.RecalculateMaxWalkSpeed`)
          (`self.MULTICAST // Recalculate WalkSpeed` (`CharacterMovementComponent.MaxWalkSpeed` (`self.CharacterMovement`))) ; In Case of Walk Speed you have to \nSet the value on Client to prevent "teleporting"
        )))))

(fn `RecalculateMaxWalkSpeed`
  (bind _returnvalue (`/Game/DRS_System/Content/DRS_System/DRS_FunctionLibrary.CalculateValue` (`self.Get BaseMaxWalkSpeed`) (`/Game/DRS_System/Content/DRS_System/Gameplay/C_GameplayEffects.Get ActiveModifier` (`self.C_GameplayEffects`)) "NewEnumerator9"))
  (`self.Is Server?`
    (:`true`
      (`/Engine/EditorBlueprintResources/StandardMacros.IsValid` (`self.C_GameplayEffects`)
        (:`Is Valid`
          (set `CharacterMovementComponent.MaxWalkSpeed` (`KismetMathLibrary.FClamp` _returnvalue 0.0 _returnvalue) (`self.CharacterMovement`)))))))

(fn `UserConstructionScript`)
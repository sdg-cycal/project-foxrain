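; Demo room graph display that plots a material-driven function with adjustable axis ranges, axis labels and an optional formula readout.
; The construction script creates the graph's dynamic material instance and applies default range, value and text.
; While an actor overlaps the capsule, Tick feeds slider values into the material and labels, packing symmetric X/Y limits into one Range vector.
; Formula text supports standard and symmetric clamp formats.
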(event `self.ReceiveTick`
  (params (DeltaSeconds :type "Float (single-precision)"))
  (bind _graphmid (`self.GraphMID`))
  (bind _functiontype (`self.FunctionType`))
  (bind _formulatext (`self.FormulaText`))
  (bind _returnvalue (`KismetTextLibrary.Conv_TextToString` (`self.Formula`)))
  (bind _returnvalue_2 (`KismetMathLibrary.Conv_IntToDouble` (`self.SliderMax`)))
  (bind _returnvalue_3 (* (`/Game/FTMagicPack01/DemoRoomData/Blueprints/BP_Slider.Value` (`self.VariableSlider`)) (`KismetMathLibrary.Conv_IntToDouble` (`self.VariableMax`))))
  (bind _returnvalue_4 (* (`/Game/FTMagicPack01/DemoRoomData/Blueprints/BP_Slider.Value` (`self.X-Slider`)) _returnvalue_2))
  (bind _returnvalue_5 (* (`/Game/FTMagicPack01/DemoRoomData/Blueprints/BP_Slider.Value` (`self.Y-Slider`)) _returnvalue_2))
  (bind _returnvalue_6 (`KismetTextLibrary.Conv_DoubleToText` _returnvalue_3 "HalfToEven" false true 1 324 1 2))
  (bind _returnvalue_7 (`KismetTextLibrary.Conv_TextToString` (`KismetTextLibrary.Conv_DoubleToText` _returnvalue_4 "HalfToEven" false true 1 324 1 1)))
  (bind _returnvalue_8 (`KismetTextLibrary.Conv_TextToString` (`KismetTextLibrary.Conv_DoubleToText` _returnvalue_5 "HalfToEven" false true 1 324 1 1)))
  (bind _returnvalue_9 (`KismetTextLibrary.Conv_TextToString` _returnvalue_6))
  (bind _returnvalue_10 (`KismetTextLibrary.Conv_TextToString` (`KismetTextLibrary.Conv_DoubleToText` (* _returnvalue_4 -1.0) "HalfToEven" false true 1 324 1 1)))
  (bind _returnvalue_11 (`KismetTextLibrary.Conv_TextToString` (`KismetTextLibrary.Conv_DoubleToText` (* _returnvalue_5 -1.0) "HalfToEven" false true 1 324 1 1)))
  (if (`self.PlayerNear`)
    (`MaterialInstanceDynamic.SetVectorParameterValue` _graphmid "Range" (make `LinearColor` (`KismetStringLibrary.Conv_StringToDouble` _returnvalue_10) (`KismetStringLibrary.Conv_StringToDouble` _returnvalue_7) (`KismetStringLibrary.Conv_StringToDouble` _returnvalue_11) (`KismetStringLibrary.Conv_StringToDouble` _returnvalue_8)))
    (if (`self.UsesVariable`)
      (`MaterialInstanceDynamic.SetScalarParameterValue` _graphmid "Value" (`KismetStringLibrary.Conv_StringToDouble` _returnvalue_9)))
    (if (`self.UsesVariable2`)
      (`MaterialInstanceDynamic.SetScalarParameterValue` _graphmid "Value2" (`/Game/FTMagicPack01/DemoRoomData/Blueprints/BP_Slider.Value` (`self.VariableSlider2`))))
    (`TextRenderComponent.SetText` (`self.X-min`) _returnvalue_10)
    (`TextRenderComponent.SetText` (`self.X-Max`) _returnvalue_7)
    (`TextRenderComponent.SetText` (`self.Y-Min`) _returnvalue_11)
    (`TextRenderComponent.SetText` (`self.Y-Max`) _returnvalue_8)
    (if (`self.ShowFormula`)
      (if (`|EnumEquality` _functiontype "NewEnumerator0")
        (if (`self.UsesVariable`)
          ;[1 1 1] Standard Variable Formula
          (`TextRenderComponent.SetText` _formulatext (`KismetStringLibrary.Concat_StrStr` (`KismetStringLibrary.Concat_StrStr` _returnvalue _returnvalue_9) ")"))
          (else
            ;[1 1 1] No Variable Formula
            (`TextRenderComponent.SetText` _formulatext _returnvalue)))
        (else
          ;[1 1 1] Clamp Formula
          (if (`|EnumEquality` _functiontype "NewEnumerator1")
            (`TextRenderComponent.SetText` (`self.FormulaText`) (`KismetStringLibrary.Concat_StrStr` (`KismetStringLibrary.Concat_StrStr` (`KismetStringLibrary.Concat_StrStr` (`KismetStringLibrary.Concat_StrStr` (`KismetTextLibrary.Conv_TextToString` (`self.Formula`)) (`KismetTextLibrary.Conv_TextToString` (`KismetTextLibrary.Conv_DoubleToText` (* _returnvalue_3 -1.0) "HalfToEven" false true 1 324 1 2))) ",") (`KismetTextLibrary.Conv_TextToString` _returnvalue_6)) ")")))))
      (else
        (`TextRenderComponent.SetText` (`self.FormulaText`) "")
        (`TextRenderComponent.SetText` (`self.Formulaheader`) "")))))

(event `self.Capsule1.OnComponentBeginOverlap`
  (params (OverlappedComponent :type "PrimitiveComponent Object Reference") (OtherActor :type "Actor Object Reference") (OtherComp :type "PrimitiveComponent Object Reference") (OtherBodyIndex :type Integer) (bFromSweep :type Boolean) (SweepResult :type "HitResult Structure (by ref)"))
  (set `self.PlayerNear` true))

(event `self.Capsule1.OnComponentEndOverlap`
  (params (OverlappedComponent :type "PrimitiveComponent Object Reference") (OtherActor :type "Actor Object Reference") (OtherComp :type "PrimitiveComponent Object Reference") (OtherBodyIndex :type Integer))
  (set `self.PlayerNear` false))

(fn `SetRange`
  (bind _returnvalue (* (`/Game/FTMagicPack01/DemoRoomData/Blueprints/BP_Slider.Value` (`self.Y-Slider`)) 10.0))
  (bind _returnvalue_2 (* (`/Game/FTMagicPack01/DemoRoomData/Blueprints/BP_Slider.Value` (`self.X-Slider`)) 10.0))
  (`MaterialInstanceDynamic.SetVectorParameterValue` (`self.GraphMID`) "Range" (make `LinearColor` (* _returnvalue_2 -1.0) _returnvalue_2 (* _returnvalue -1.0) _returnvalue)))

(fn `UserConstructionScript`
  (bind _graphmid (`self.GraphMID`))
  (bind _default_range (`self.Default Range`))
  (bind _functiontype (`self.FunctionType`))
  (bind _formulatext (`self.FormulaText`))
  (bind _variabledefault (`self.VariableDefault`))
  (bind (_r _g _b _a) (break `LinearColor` _default_range))
  (bind _returnvalue (`PrimitiveComponent.CreateDynamicMaterialInstance` (`self.GraphMesh`) 0 (`self.Graph Material`) "None"))
  (set `self.GraphMID` _returnvalue)
  (`MaterialInstanceDynamic.SetVectorParameterValue` _graphmid "Range" _default_range)
  (`MaterialInstanceDynamic.SetScalarParameterValue` _graphmid "Value" (`self.VariableDefault`))
  (`TextRenderComponent.SetText` (`self.X-min`) (`KismetStringLibrary.Conv_DoubleToString` _r))
  (`TextRenderComponent.SetText` (`self.X-Max`) (`KismetStringLibrary.Conv_DoubleToString` _g))
  (`TextRenderComponent.SetText` (`self.Y-Min`) (`KismetStringLibrary.Conv_DoubleToString` _b))
  (`TextRenderComponent.SetText` (`self.Y-Max`) (`KismetStringLibrary.Conv_DoubleToString` _a))
  (if (`self.ShowFormula`)
    (if (`|EnumEquality` _functiontype "NewEnumerator0")
      (if (`self.UsesVariable`)
        ;[1 1 1] Standard Variable formula
        (`TextRenderComponent.SetText` _formulatext (`KismetStringLibrary.Concat_StrStr` (`KismetStringLibrary.Concat_StrStr` (`KismetTextLibrary.Conv_TextToString` (`self.Formula`)) (`KismetStringLibrary.Conv_DoubleToString` (`self.VariableDefault`))) ")"))
        (else
          ;[1 1 1] No Variable Formula
          (`TextRenderComponent.SetText` _formulatext (`KismetTextLibrary.Conv_TextToString` (`self.Formula`)))))
      (elif (`|EnumEquality` _functiontype "NewEnumerator1")
        ;[1 1 1] Clamp Formula
        (`TextRenderComponent.SetText` (`self.FormulaText`) (`KismetStringLibrary.Concat_StrStr` (`KismetStringLibrary.Concat_StrStr` (`KismetStringLibrary.Concat_StrStr` (`KismetStringLibrary.Concat_StrStr` (`KismetTextLibrary.Conv_TextToString` (`self.Formula`)) (`KismetStringLibrary.Conv_DoubleToString` (* _variabledefault -1.0))) ",") (`KismetStringLibrary.Conv_DoubleToString` _variabledefault)) ")"))))
    (else
      (`TextRenderComponent.SetText` (`self.Formulaheader`) "")
      (`TextRenderComponent.SetText` (`self.FormulaText`) ""))))
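; Cull volume actor for the GoodRain system that publishes a world-aligned region to the MPC_GR_ParameterCollection material parameter collection.
; Init runs on construction and BeginPlay, locking rotation to zero and writing the actor location and absolute scale times 100 as Cull Location and Cull Radius.
; It also applies the HiddenInGame flag to the Cube component.
; Destroying the actor resets both collection parameters to zero.
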(event `self.ReceiveBeginPlay`
  (`self.Init`))

(event `self.ReceiveTick`
  (params (DeltaSeconds :type "Float (single-precision)")))

(event `self.ReceiveDestroyed`
  (bind _returnvalue (`KismetMathLibrary.Conv_VectorToLinearColor` (`KismetMathLibrary.MakeVector` 0.0)))
  ;[1 1 1] Reset value
  (`KismetMaterialLibrary.SetVectorParameterValue` "/Game/GoodRain/Sources/Materials/MatCollection/MPC_GR_ParameterCollection.MPC_GR_ParameterCollection" "Cull Location" _returnvalue)
  (`KismetMaterialLibrary.SetVectorParameterValue` "/Game/GoodRain/Sources/Materials/MatCollection/MPC_GR_ParameterCollection.MPC_GR_ParameterCollection" "Cull Radius" _returnvalue))

(fn `Init`
  ;[1 1 1] Lock Rotation
  (`SceneComponent.K2_SetWorldRotation` :`self` (`self.DefaultSceneRoot`))
  ;[1 1 1] Get Cull Actor Location / Scale
  (`KismetMaterialLibrary.SetVectorParameterValue` "/Game/GoodRain/Sources/Materials/MatCollection/MPC_GR_ParameterCollection.MPC_GR_ParameterCollection" "Cull Location" (`KismetMathLibrary.Conv_VectorToLinearColor` (`self.K2_GetActorLocation`)))
  (`KismetMaterialLibrary.SetVectorParameterValue` "/Game/GoodRain/Sources/Materials/MatCollection/MPC_GR_ParameterCollection.MPC_GR_ParameterCollection" "Cull Radius" (`KismetMathLibrary.Conv_VectorToLinearColor` (* (`KismetMathLibrary.MakeVector` (`KismetMathLibrary.Abs` (.x (`SceneComponent.K2_GetComponentScale` (`self.DefaultSceneRoot`)))) (`KismetMathLibrary.Abs` (.y (`SceneComponent.K2_GetComponentScale` (`self.DefaultSceneRoot`)))) (`KismetMathLibrary.Abs` (.z (`SceneComponent.K2_GetComponentScale` (`self.DefaultSceneRoot`))))) (100.0 100.0 100.0))))
  ;[1 1 1] Check bool
  (`SceneComponent.SetHiddenInGame` (`self.Cube`) (`self.Hidden In Game`) false))

(fn `UserConstructionScript`
  (`self.Init`))
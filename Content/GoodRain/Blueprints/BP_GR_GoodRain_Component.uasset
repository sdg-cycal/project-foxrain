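; GoodRain component that adds rain particles, looping sound and ground splashes around its owning actor.
; BeginPlay and a toggle event spawn the attached effects and push rain settings into a Material Parameter Collection, which an update event refreshes; toggling off removes them.
; A Delay-driven loop fires random downward line traces around the owner, spawning splash or ripple emitters at hits, timed by rain amount and frequency, with optional debug drawing.
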(event `Good Rain Update Event`
  (`self.valueSetting`))

(event `self.ReceiveTick`
  (params (DeltaSeconds :type "Float (single-precision)")))

(event `Good Rain Toggle Event`
  (bind _returnvalue (`self.GetOwner`))
  (bind _area_of_splash_ (`self.Area of Splash `))
  (bind _returnvalue_2 (`Actor.K2_GetActorLocation` _returnvalue))
  (bind _returnvalue_3 (* _area_of_splash_ -1.0))
  (bind _returnvalue_4 (/ 1.0 (* (`self.Amount of Rain`) (`self.Frequency of Splash `))))
  (bind _z (.z _returnvalue_2))
  (bind _returnvalue_5 (`KismetStringLibrary.Conv_DoubleToString` (/ (* _area_of_splash_ 2.0) 100.0)))
  (bind _returnvalue_6 (+ (.y _returnvalue_2) (`KismetMathLibrary.RandomFloatInRange` _returnvalue_3 _area_of_splash_)))
  (bind _returnvalue_7 (+ (.x _returnvalue_2) (`KismetMathLibrary.RandomFloatInRange` _returnvalue_3 _area_of_splash_)))
  (if (`self.Enable Rain System`)
    (`|ExecutionSequence` :!label _label
      (:`then_0`
        ;[1 1 1] Debug String
        (if (`self.Enable Debug Mode`)
          (`KismetSystemLibrary.PrintString` (`KismetStringLibrary.Concat_StrStr` "splash Number :" (`KismetStringLibrary.Conv_IntToString` (`self.Mutiple of Splash`)) " / " (`KismetStringLibrary.Conv_DoubleToString` _returnvalue_4) "second" " in " _returnvalue_5 " m x " _returnvalue_5 " m ") true false (struct :`G` 0.66 :`B` 1.0 :`A` 1.0) 60.0)))
      (:`then_1`
        (if (`self.Enable Rain System`)
          (if (`self.Enable Sound`)
            ;[1 1 1] Sound Setting
            (bind _returnvalue_8 (`GameplayStatics.SpawnSoundAttached` "/Game/GoodRain/Sources/Audio/Cue/SC_GR_Rain_Loop.SC_GR_Rain_Loop" (`Actor.RootComponent` _returnvalue) "None" _returnvalue_2 (struct) "KeepWorldPosition" false (`KismetMathLibrary.FClamp` (`self.Amount of Rain`) 0.3 0.9) 1.0 0.0 null null)))
          ;[1 1 1] Rain FX
          (bind _returnvalue_9 (`GameplayStatics.SpawnEmitterAttached` "/Game/GoodRain/Sources/Particles/PS_GR_Rain.PS_GR_Rain" (`Actor.RootComponent` _returnvalue) "None" _returnvalue_2 (struct) (1.0 1.0 1.0) "KeepWorldPosition"))
          ;[1 1 1] Rotation
          (`ParticleSystemComponent.SetVectorParameter` _returnvalue_9 "Rain Rotation" (`KismetMathLibrary.MakeVector` (`self.Rain Tilt Intensity`)))
          (`self.valueSetting`)
          ;[1 1 1] check Boolean
          (if (`self.Enable Splash`)
            ;[1 1 1] Splash FX Loop
            (for _ (range 1 (+ (`self.Mutiple of Splash`) 1)) :!label _label_2
              (if (`self.Enable Rain System`)
                (bind (_outhit _returnvalue_10) (`KismetSystemLibrary.LineTraceSingle` :`Start` (`KismetMathLibrary.MakeVector` _returnvalue_7 _returnvalue_6 (+ _z 20000.0)) :`End` (`KismetMathLibrary.MakeVector` _returnvalue_7 _returnvalue_6 (+ _z -10000.0)) :`TraceChannel` "TraceTypeQuery1" :`bTraceComplex` (`self.Enable Splash Hit TraceComplex`) :`DrawTime` 0.1))
                (if _returnvalue_10
                  (if (`self.Enable Debug Mode`)
                    (bind (_bblockinghit _binitialoverlap _time _distance _location _impactpoint _normal _impactnormal _physmat _hitactor _hitcomponent _hitbonename _bonename _hititem _elementindex _faceindex _tracestart _traceend) (`GameplayStatics.BreakHitResult` _outhit))
                    (`KismetSystemLibrary.DrawDebugLine` _tracestart _traceend (struct :`R` 1.0 :`A` 1.0) 0.1 2.0)
                    (`KismetSystemLibrary.DrawDebugSphere` _location 12.0 12 (struct :`R` 1.0 :`A` 1.0) 0.1 2.0))
                  (if (`self.Enable Splash With Ripple`)
                    (`GameplayStatics.SpawnEmitterAtLocation` "/Game/GoodRain/Sources/Particles/PS_GR_Splash_Ripple.PS_GR_Splash_Ripple" _location)
                    (else
                      (`GameplayStatics.SpawnEmitterAtLocation` "/Game/GoodRain/Sources/Particles/PS_GR_Splash.PS_GR_Splash" _location))))
                (`KismetSystemLibrary.Delay` _returnvalue_4 :!label _label_3)
                (goto _label_2)))
            (goto _label_3)
            (else
              ;[1 1 1] force uncheck
              (set `self.Enable Splash With Ripple` false))))))
    (else
      (`self.K2_DestroyComponent` _returnvalue_9)
      (`AudioComponent.Stop` _returnvalue_8))))

(event `self.ReceiveBeginPlay`
  (goto _label))

(fn `valueSetting`
  ;[1 1 1] MPC Setting
  (`KismetMaterialLibrary.SetScalarParameterValue` "/Game/GoodRain/Sources/Materials/MatCollection/MPC_GR_ParameterCollection.MPC_GR_ParameterCollection" "Global Drop Speed" (`self.Rain Drop Speed`))
  (`KismetMaterialLibrary.SetScalarParameterValue` "/Game/GoodRain/Sources/Materials/MatCollection/MPC_GR_ParameterCollection.MPC_GR_ParameterCollection" "Global Amount of Rain" (`self.Amount of Rain`))
  (`KismetMaterialLibrary.SetScalarParameterValue` "/Game/GoodRain/Sources/Materials/MatCollection/MPC_GR_ParameterCollection.MPC_GR_ParameterCollection" "Global Refraction Intensity" (`self.Global Refraction Intensity`))
  (`KismetMaterialLibrary.SetScalarParameterValue` "/Game/GoodRain/Sources/Materials/MatCollection/MPC_GR_ParameterCollection.MPC_GR_ParameterCollection" "Global Opacity Intensity" (`self.Global Opacity Intensity`))
  (`KismetMaterialLibrary.SetVectorParameterValue` "/Game/GoodRain/Sources/Materials/MatCollection/MPC_GR_ParameterCollection.MPC_GR_ParameterCollection" "Global Base Color" (`self.Global Base Color`)))